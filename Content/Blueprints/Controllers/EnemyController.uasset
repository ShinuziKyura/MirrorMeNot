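; AI controller for enemies that runs the EnemyBT behavior tree and tracks whether the player can be seen.
; AI Perception updates for the PaperPlayer set the CanSeePlayer blackboard key, true only when the stimulus is sensed and IsPlayerVisible is set.
; The game mode's OnWorldsShifted event clears IsPlayerVisible when worlds are reversed and restores it otherwise, reaching the blackboard only on the next perception update.
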(event OnTargetPerceptionUpdated(AIPerception)
  (params (Actor :type Actor%20Object%20Reference) (Stimulus :type AI%20Stimulus%20Structure))
  (Utilities|Casting|CastToPaperPlayer Actor)
  (AI|Components|Blackboard|SetValueasBool (AI|GetBlackboard 0) (Utilities|Name|MakeLiteralName "CanSeePlayer") (and (.bSuccessfullySensed (Utilities|Struct|BreakAIStimulus Stimulus)) (Variables|Default|GetIsPlayerVisible))))

(event Custom|Event%20On%20Worlds%20Shifted
  (params (bReversed :type Boolean))
  (Variables|Default|SetIsPlayerVisible (not bReversed)))

(event EventBeginPlay
  (AI|RunBehaviorTree "/Game/Behaviour/PaperEnemy/EnemyBT.EnemyBT")
  (bind _asmirror_me_not_game_mode_base (Utilities|Casting|CastToMirrorMeNotGameModeBase (Game|GetGameMode)))
  (EventDispatchers|BindEventtoOnWorldsShifted _asmirror_me_not_game_mode_base (delegate Custom|Event%20On%20Worlds%20Shifted)))

(fn ConstructionScript)